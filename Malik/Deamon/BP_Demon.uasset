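; BP_Demon is a demon enemy pawn that pursues the player once spotted and can play a catch animation.
; PawnSensing sets a seen flag, which the FollowPlayer event checks before moving the demon to the player with AIMoveTo.
; FollowPlayer clears CanGrab first, so the catch animation and following delay run only if that flag is set again before the move succeeds.
; Nothing in this graph sets CanGrab true or calls FollowPlayer.
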(event OnSeePawn(PawnSensing)
  (params (Pawn :type Pawn%20Object%20Reference))
  (Variables|Default|SetIsSeenPlayer true))

(event Custom|Follow%20Player
  (Variables|Default|SetCanGrab false)
  (if (Variables|Default|GetIsSeenPlayer)
    (AI|AIMoveTo self "0, 0, 0" (Game|GetPlayerCharacter 0) 5.0 false
      (:OnSuccess
        (if (Variables|Default|GetCanGrab)
          (Variables|Default|SetCanGrab false)
          (Components|Animation|PlayAnimation (Variables|Character|GetMesh) "/Game/Vadi/Malik/Deamon/demon_catch.demon_catch" false)
          (Utilities|FlowControl|Delay 3.71))))
    (else
      (Variables|Default|SetIsSeenPlayer false))))

(event EventBeginPlay)

(event Collision|EventActorBeginOverlap
  (params (OtherActor :type Actor%20Object%20Reference)))

(event EventTick
  (params (DeltaSeconds :type Float%20%28single-precision%29)))

(fn ConstructionScript)